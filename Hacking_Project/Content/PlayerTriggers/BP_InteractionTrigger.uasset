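; Player trigger for a lockable interaction, showing a prompt on the HUD of the player inside it.
; Entering or exiting shows or hides the prompt, built from lock state, interaction text and the first Enhanced Input key mapped to IA_Interact.
; TryInteract starts the interaction only when unlocked, and lock changes refresh the HUD while a player is inside.
; Start and end handlers only print debug messages, and a debug event toggles the lock.
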(event `DBG_ToggleLock`
  (`self.UnlockInteraction` (`self.bIsLocked`)))

(fn `GetInteractionKey`
  (returns (ReturnValue :type String))
  (bind _returnvalue (pcsubsystem `EnhancedInputLocalPlayerSubsystem` (`GameplayStatics.GetPlayerController` 0)))
  (`/Engine/EditorBlueprintResources/StandardMacros.IsValid` _returnvalue
    (:`Is Valid`
      (return (`KismetTextLibrary.Conv_TextToString` (`KismetInputLibrary.Key_GetDisplayName` (`|GetArrayItem` (`EnhancedInputSubsystemInterface.QueryKeysMappedToAction` _returnvalue "/Game/_Core/Input/Actions/IA_Interact.IA_Interact"))))))
    (:`Is Not Valid`
      (return "INVALID"))))

(fn `GetInteractionText`
  (returns (Text :type String))
  (return (`self.InteractionText`)))

(fn `OnInteractionEnd`
  (`KismetSystemLibrary.PrintString` (`KismetStringLibrary.Concat_StrStr` (`KismetSystemLibrary.GetDisplayName` self) " | Interaction END") true true (struct :`R` 1.0 :`G` 0.461012 :`A` 1.0)))

(fn `OnInteractionStart`
  (`KismetSystemLibrary.PrintString` (`KismetStringLibrary.Concat_StrStr` (`KismetSystemLibrary.GetDisplayName` self) " | Interaction START") true true (struct :`G` 1.0 :`B` 0.158936 :`A` 1.0)))

(fn `OnPlayerEnter`
  (`parent.OnPlayerEnter`)
  (`self.RefreshHUD` true))

(fn `OnPlayerExit`
  (`parent.OnPlayerExit`)
  (`self.RefreshHUD` false))

(fn `RefreshHUD`
  (params (bDisplay :type Boolean))
  (`/Game/UI/WBP_PlayerHUD.DisplayInteraction` (`/Game/Player/BP_Player.HUDWidget` (`self.PlayerInTrigger`)) bDisplay (`self.bIsLocked`) (`self.GetInteractionText`) (`self.GetInteractionKey`)))

(fn `TryInteract`
  (if (not (`self.bIsLocked`))
    (`self.OnInteractionStart`)))

(fn `UnlockInteraction`
  (params (bUnlock :type Boolean))
  (set `self.bIsLocked` (not bUnlock))
  (`self.PlayerInTrigger`
    (:`then`
      (`self.RefreshHUD` true))
    (:`else`)))

(fn `UserConstructionScript`
  (`parent.UserConstructionScript`))