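; BP_PlayerTrigger is a base trigger volume that detects when a BP_Player enters or leaves its Collision component.
; Begin and end overlap events filter for BP_Player, track it in PlayerInTrigger and route to OnPlayerEnter and OnPlayerExit.
; Those functions print debug messages and notify the player through OnTriggerEnter, passing the trigger itself, and OnTriggerExit.
; PlayerInTrigger clears after the exit notification.
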(event `self.Collision.OnComponentBeginOverlap`
  (params (OverlappedComponent :type "PrimitiveComponent Object Reference") (OtherActor :type "Actor Object Reference") (OtherComp :type "PrimitiveComponent Object Reference") (OtherBodyIndex :type Integer) (bFromSweep :type Boolean) (SweepResult :type "HitResult Structure (by ref)"))
  (bind _asbp_player (cast `/Game/Player/BP_Player` OtherActor))
  (set `self.PlayerInTrigger` _asbp_player)
  (`self.OnPlayerEnter`))

(event `self.Collision.OnComponentEndOverlap`
  (params (OverlappedComponent :type "PrimitiveComponent Object Reference") (OtherActor :type "Actor Object Reference") (OtherComp :type "PrimitiveComponent Object Reference") (OtherBodyIndex :type Integer))
  (cast `/Game/Player/BP_Player` OtherActor)
  (`self.OnPlayerExit`)
  (set `self.PlayerInTrigger` null))

(fn `OnPlayerEnter`
  (`KismetSystemLibrary.PrintString` (`KismetStringLibrary.Concat_StrStr` (`KismetSystemLibrary.GetDisplayName` self) " | Player ENTER"))
  (`/Game/Player/BP_Player.OnTriggerEnter` (`self.PlayerInTrigger`) self))

(fn `OnPlayerExit`
  (`KismetSystemLibrary.PrintString` (`KismetStringLibrary.Concat_StrStr` (`KismetSystemLibrary.GetDisplayName` self) " | Player EXIT") true true (struct :`R` 1.0 :`G` 0.414137 :`A` 1.0))
  (`/Game/Player/BP_Player.OnTriggerExit` (`self.PlayerInTrigger`)))

(fn `UserConstructionScript`)