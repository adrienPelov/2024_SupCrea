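; BP_YOLO is a test Blueprint that slides along world X as it ticks.
; Tick calls UpdateMovement, which adds Speed to the root's location each frame without delta-time scaling; its branch is fixed false, so the Y path never runs and RandomBool sits unused.
; DisplayTime, which prints an accumulated time, and UpdateScale, which stretches Visual along X, are defined but not called here.
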(event `self.ReceiveBeginPlay`
  (`KismetSystemLibrary.PrintString` "Start"))

(event `self.ReceiveTick`
  (params (DeltaSeconds :type "Float (single-precision)"))
  (`self.UpdateMovement`))

(fn `DisplayTime`
  (params (Time :type "Float (double-precision)"))
  (bind _output_get (set `self.TotalTime` (+ Time (`self.TotalTime`))))
  (`KismetSystemLibrary.PrintString` (`KismetStringLibrary.Concat_StrStr` "Total Time - " (`KismetStringLibrary.Conv_DoubleToString` _output_get)) true true (struct :`R` 0.026884 :`G` 1.0 :`A` 1.0)))

(fn `UpdateMovement`
  (bind _defaultsceneroot (`self.DefaultSceneRoot`))
  (bind (_returnvalue_x _returnvalue_y _returnvalue_z) (`KismetMathLibrary.BreakVector` (`SceneComponent.K2_GetComponentLocation` _defaultsceneroot)))
  (if false
    (`SceneComponent.K2_SetWorldLocation` _defaultsceneroot (`KismetMathLibrary.MakeVector` _returnvalue_x (+ (`self.Speed`) _returnvalue_y) _returnvalue_z) false false)
    (else
      (`SceneComponent.K2_SetWorldLocation` _defaultsceneroot (`KismetMathLibrary.MakeVector` (+ _returnvalue_x (`self.Speed`)) _returnvalue_y _returnvalue_z) false false))))

(fn `UpdateScale`
  (bind _visual (`self.Visual`))
  (`SceneComponent.SetWorldScale3D` _visual (`KismetMathLibrary.MakeVector` (+ (.x (`SceneComponent.K2_GetComponentScale` _visual)) 0.1) (.y (`SceneComponent.K2_GetComponentScale` _visual)) (.z (`SceneComponent.K2_GetComponentScale` _visual)))))

(fn `UserConstructionScript`)