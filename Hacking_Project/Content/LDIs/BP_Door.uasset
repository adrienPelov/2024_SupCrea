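; BP_Door is an interactable sliding door that toggles between open and closed, with a matching "Open" or "Close" prompt.
; Construction caches positions from two target components, with names crossed (TargetOpen feeds PositionClose), and snaps VisualRoot to the IsOpen state.
; Interaction plays or reverses a timeline, rate-scaled by TimeToOpen, that lerps VisualRoot with sweep.
; When the timeline finishes, interaction ends, flipping IsOpen and refreshing the HUD.
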(event `self.ReceiveBeginPlay`
  (`parent.ReceiveBeginPlay`)
  (`self.InitTime`))

(event `Evt_Open`
  (bind (_direction _interpolation) (`Timeline|TimeLineOpenDoor` :!label _label)
    (:`Update`
      (`SceneComponent.K2_SetRelativeLocation` (`self.VisualRoot`) (`KismetMathLibrary.VLerp` (`self.PositionClose`) (`self.PositionOpen`) _interpolation) true false))
    (:`Finished`
      (`self.OnInteractionEnd`))))

(event `Evt_Close`
  (goto _label :!via `Reverse`))

(fn `GetInteractionText`
  (returns (Text :type String))
  (if (`self.bIsOpen`)
    (return "Close")
    (else
      (return "Open"))))

(fn `InitPosition`
  (bind _visualroot (`self.VisualRoot`))
  (`|ExecutionSequence`
    (:`then_0`
      (set `self.PositionClose` (`SceneComponent.RelativeLocation` (`self.TargetOpen`))))
    (:`then_1`
      (set `self.PositionOpen` (`SceneComponent.RelativeLocation` (`self.TargetClose`))))
    (:`then_2`
      (if (`self.bIsOpen`)
        (`SceneComponent.K2_SetRelativeLocation` _visualroot (`self.PositionOpen`) false true)
        (else
          (`SceneComponent.K2_SetRelativeLocation` _visualroot (`self.PositionClose`) false true))))))

(fn `InitTime`
  (`TimelineComponent.SetPlayRate` (`self.TimeLineOpenDoor`) (/ 1.0 (`self.TimeToOpen`))))

(fn `OnInteractionEnd`
  (`parent.OnInteractionEnd`)
  (if (`self.bIsOpen`)
    (set `self.bIsOpen` false)
    (else
      (set `self.bIsOpen` true)))
  (`self.RefreshHUD` true))

(fn `OnInteractionStart`
  (`parent.OnInteractionStart`)
  (if (`self.bIsOpen`)
    (`self.Evt_Close`)
    (else
      (`self.Evt_Open`))))

(fn `UserConstructionScript`
  (`parent.UserConstructionScript`)
  (`self.InitPosition`))