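; BP_HackTarget is an interactable actor that the player can hack, showing "Hack" as its interaction text.
; When interaction starts, it selects the Easy, Medium or Hard settings according to its Difficulty value.
; It then passes those settings to BP_PlayerController on player index 0 to activate hacking mode.
; The hacking itself is not implemented here, and the event graph holds only disabled placeholder events.
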(fn `GetInteractionText`
  (returns (Text :type String))
  (return "Hack"))

(fn `OnInteractionStart`
  (locals (L_settings :type "/Game/Hacking/_Structs/FHackingSetting Structure"))
  (`parent.OnInteractionStart`)
  (switch `/Game/Hacking/_Enums/EHackingDifficulty` (`self.Difficulty`)
    (:`NewEnumerator0`
      (set `local.L_settings` (`self.SettingsEasy`)))
    (:`NewEnumerator1`
      (set `local.L_settings` (`self.SettingsMedium`)))
    (:`NewEnumerator2`
      (set `local.L_settings` (`self.SettingsHard`))))
  (bind _asbp_player_controller (cast `/Game/Player/BP_PlayerController` (`GameplayStatics.GetPlayerController` 0)))
  (`/Game/Player/BP_PlayerController.ActivateHackingMode` _asbp_player_controller true (`local.L_settings`)))

(fn `UserConstructionScript`
  (`parent.UserConstructionScript`))