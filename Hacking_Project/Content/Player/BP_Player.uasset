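; Player character Blueprint that handles walk and sprint movement, stamina and trigger-based interaction.
; BeginPlay applies movement and jump settings, fills stamina and creates the HUD widget.
; Tick drains stamina while sprinting, dropping to walk speed when empty, otherwise regenerates it, and pushes the value to the HUD.
; Trigger enter and exit functions track the current trigger, which Interact casts to BP_TriggerInteraction to attempt interaction.
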(event `self.ReceiveBeginPlay`
  (`self.InitPlayer`))

(event `self.ReceiveTick`
  (params (DeltaSeconds :type "Float (single-precision)"))
  (`self.UpdatePlayer` DeltaSeconds))

(fn `InitCharacterMovement`
  (bind _charactermovement (`self.CharacterMovement`))
  (`|ExecutionSequence`
    (:`then_0`
      (set `CharacterMovementComponent.MaxWalkSpeed` (`self.SpeedWalk`) _charactermovement))
    (:`then_1`
      (set `CharacterMovementComponent.JumpZVelocity` (`self.JumpForce`) _charactermovement))
    (:`then_2`
      (set `CharacterMovementComponent.AirControl` (`self.JumpAirControl`) _charactermovement))))

(fn `InitPlayer`
  (`|ExecutionSequence`
    (:`then_0`
      (`self.InitCharacterMovement`))
    (:`then_1`
      (set `self.Stamina` (`self.StaminaMax`)))
    (:`then_2`
      (set `self.bSprint` false))
    (:`then_3`
      (bind _returnvalue (`|CreateWidget` "/Game/UI/WBP_PlayerHUD.WBP_PlayerHUD_C"))
      (bind _output_get (set `self.HUDWidget` _returnvalue))
      (`UserWidget.AddToPlayerScreen` _output_get 0))))

(fn `Interact`
  (bind _asbp_interaction_trigger (cast `/Game/PlayerTriggers/BP_TriggerInteraction` (`self.CurrentTrigger`)))
  (`/Game/PlayerTriggers/BP_TriggerInteraction.TryInteract` _asbp_interaction_trigger))

(fn `OnTriggerEnter`
  (params (NewTrigger :type "/Game/PlayerTriggers/_Base/BP_TriggerPlayer Object Reference"))
  (set `self.CurrentTrigger` NewTrigger))

(fn `OnTriggerExit`
  (set `self.CurrentTrigger` null))

(fn `Sprint`
  (params (bSprint :type Boolean))
  (bind _charactermovement (`self.CharacterMovement`))
  (bind _output_get (set `self.bSprint` bSprint))
  (if _output_get
    (set `CharacterMovementComponent.MaxWalkSpeed` (`self.SpeedSprint`) _charactermovement)
    (else
      (set `CharacterMovementComponent.MaxWalkSpeed` (`self.SpeedWalk`) _charactermovement))))

(fn `UpdatePlayer`
  (params (deltaTime :type "Float (double-precision)"))
  (`|ExecutionSequence`
    (:`then_0`
      (`self.UpdateStamina` deltaTime))))

(fn `UpdateStamina`
  (params (deltaTime :type "Float (double-precision)"))
  (bind _staminamax (`self.StaminaMax`))
  (if (`self.bSprint`)
    (set `self.Stamina` (`KismetMathLibrary.FClamp` (- (`self.Stamina`) deltaTime) 0.0 _staminamax))
    (`self.Sprint` (> (`self.Stamina`) 0.0))
    (else
      (set `self.Stamina` (`KismetMathLibrary.FClamp` (+ deltaTime (`self.Stamina`)) 0.0 _staminamax))))
  (`/Game/UI/WBP_PlayerHUD.UpdateStamina` (`self.HUDWidget`) (`self.Stamina`) (`self.StaminaMax`)))

(fn `UserConstructionScript`)