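; BPC_ObjectiveTarget is an actor component that marks its owner as an objective target and reports when that target is completed.
; InitTarget stores the target type and, for the Interact type, casts the owner to BP_TriggerInteraction and binds to its interaction-end dispatcher.
; OnTargetComplete fires the TargetComplete dispatcher with itself and prints a debug message naming the owner.
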(fn `InitTarget`
  (params (Type :type "/Game/Objectives/_Enums/EObjectiveType Enum" :default "NewEnumerator0"))
  (locals (L_parent :type "Actor Object Reference"))
  (set `self.Type` Type)
  (set `local.L_parent` (`self.GetOwner`))
  (switch `/Game/Objectives/_Enums/EObjectiveType` (`self.Type`)
    (:`NewEnumerator1`
      (bind _asbp_trigger_interaction (cast `/Game/PlayerTriggers/BP_TriggerInteraction` (`local.L_parent`)))
      (add `/Game/PlayerTriggers/BP_TriggerInteraction.EvtDispatcher_OnInteractionEnd` _asbp_trigger_interaction (`|CreateDelegate` :!event `OnTargetComplete`)))))

(fn `OnTargetComplete`
  (`self.EvtDispatcher_TargetComplete` self)
  (`KismetSystemLibrary.PrintString` (`KismetStringLibrary.Concat_StrStr` (`KismetSystemLibrary.GetDisplayName` (`self.GetOwner`)) " | Interaction Target Complete") true true (struct :`R` 0.91406 :`G` 0.276435 :`B` 1.0 :`A` 1.0)))