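; Objective manager that runs a level's objectives in sequence, each completed through target actors carrying BPC_ObjectiveTarget components.
; BeginPlay registers all targets and binds their completion dispatchers; only current-objective targets count toward progress.
; Tick polls for the player's HUD widget, then binds its fade-out dispatcher and starts the first objective.
; Completion updates the HUD, whose fade-out triggers the next objective; the last just prints level complete and sets a flag.
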(event `self.ReceiveBeginPlay`
  (`self.InitObjectives`))

(event `self.ReceiveTick`
  (params (DeltaSeconds :type "Float (single-precision)"))
  (`self.HUDRef`
    (:`then`)
    (:`else`
      (bind _asbp_player (cast `/Game/Player/BP_Player` (`Controller.K2_GetPawn` (`GameplayStatics.GetPlayerController` 0))))
      (bind _output_get (set `self.HUDRef` (`/Game/Player/BP_Player.HUDWidget` _asbp_player)))
      (`/Engine/EditorBlueprintResources/StandardMacros.IsValid` _output_get
        (:`Is Valid`
          (`|ExecutionSequence`
            (:`then_0`
              (add `/Game/UI/WBP_PlayerHUD.Dispatcher_FadeOutComplete` (`self.HUDRef`) (`|CreateDelegate` :!event `OnHUDFadeOutComplete`)))
            (:`then_1`
              (`self.StartObjective` 0))))))))

(fn `InitObjectives`
  (`|ExecutionSequence`
    (:`then_0`
      (set `self.CurObjectiveIndex` 0))
    (:`then_1`
      (set `self.NbTargetsComplete` 0))
    (:`then_2`
      (set `self.bAllObjCompleted` false))
    (:`then_3`
      (`KismetArrayLibrary.Array_Clear` (`self.CurTargets`)))
    (:`then_4`
      (for _array_element (`self.Objectives`)
        (bind ((`Type_7_EFA8C0FF4A7EC4CE50EFF4AA37EB1FD7` _type) (`TargetActors_15_9F57A91946992FC3A4700EBA8900627E` _targetactors)) (break `/Game/Objectives/_Structs/FObjective` _array_element))
        (for _array_element_2 _targetactors
          (bind _returnvalue (`self.GetComponentByClass` _array_element_2 "/Game/Objectives/BPC_ObjectiveTarget.BPC_ObjectiveTarget_C"))
          (`/Engine/EditorBlueprintResources/StandardMacros.IsValid` _returnvalue
            (:`Is Valid`
              (`self.RegisterTarget` _returnvalue _type))))))))

(fn `OnHUDFadeOutComplete`
  (if (not (`self.bAllObjCompleted`))
    (`self.StartObjective` (`self.CurObjectiveIndex`))))

(fn `OnObjectiveComplete`
  (`/Game/UI/WBP_PlayerHUD.CompleteObjective` (`self.HUDRef`))
  (if (< (`self.CurObjectiveIndex`) (- (`KismetArrayLibrary.Array_Length` (`self.Objectives`)) 1))
    (`/Engine/EditorBlueprintResources/StandardMacros.IncrementInt` (`self.CurObjectiveIndex`))
    (else
      (`KismetSystemLibrary.PrintString` "[Objective Manager] LEVEL -> Complete!" true true (struct :`R` 1.0 :`B` 0.120237 :`A` 1.0))
      (set `self.bAllObjCompleted` true))))

(fn `OnTargetComplete`
  (params (Target :type "/Game/Objectives/BPC_ObjectiveTarget Object Reference"))
  (if (`KismetArrayLibrary.Array_Contains` (`self.CurTargets`) Target)
    (`|ExecutionSequence`
      (:`then_0`
        (`/Engine/EditorBlueprintResources/StandardMacros.IncrementInt` (`self.NbTargetsComplete`)))
      (:`then_1`
        (`/Game/UI/WBP_PlayerHUD.UpdateObjectiveTargets` (`self.HUDRef`) (`self.NbTargetsComplete`)))
      (:`then_2`
        (if (== (`self.NbTargetsComplete`) (`KismetArrayLibrary.Array_Length` (`self.CurTargets`)))
          (`self.OnObjectiveComplete`))))))

(fn `RegisterTarget`
  (params (Target :type "/Game/Objectives/BPC_ObjectiveTarget Object Reference") (Type :type "/Game/Objectives/_Enums/EObjectiveType Enum" :default "NewEnumerator0"))
  (`|ExecutionSequence`
    (:`then_0`
      (`/Game/Objectives/BPC_ObjectiveTarget.InitTarget` Target Type))
    (:`then_1`
      (add `/Game/Objectives/BPC_ObjectiveTarget.EvtDispatcher_TargetComplete` Target (`|CreateDelegate` :!event `OnTargetComplete`)))))

(fn `StartObjective`
  (params (ObjectiveIndex :type Integer))
  (bind (_title _description _type _targetactors) (break `/Game/Objectives/_Structs/FObjective` (`|GetArrayItem` (`self.Objectives`) (`self.CurObjectiveIndex`))))
  (`|ExecutionSequence`
    (:`then_0`
      (`KismetArrayLibrary.Array_Clear` (`self.CurTargets`)))
    (:`then_1`
      (set `self.NbTargetsComplete` 0))
    (:`then_2`
      (for _array_element (`.TargetActors_15_9F57A91946992FC3A4700EBA8900627E` (break `/Game/Objectives/_Structs/FObjective` (`|GetArrayItem` (`self.Objectives`) ObjectiveIndex)))
        (bind _returnvalue (`self.GetComponentByClass` _array_element "/Game/Objectives/BPC_ObjectiveTarget.BPC_ObjectiveTarget_C"))
        (`/Engine/EditorBlueprintResources/StandardMacros.IsValid` _returnvalue
          (:`Is Valid`
            (`KismetArrayLibrary.Array_Add` (`self.CurTargets`) _returnvalue))))
      (bind _hudref (`self.HUDRef`)
        (:`then`
          (`/Game/UI/WBP_PlayerHUD.StartObjective` _hudref _type _title _description (`KismetArrayLibrary.Array_Length` _targetactors)))
        (:`else`)))))

(fn `UserConstructionScript`)